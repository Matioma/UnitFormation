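; BP_RPSController is a player controller that lets the player click in the world to set a destination for a BP_Unit.
; On BeginPlay it sets game-and-UI input with a locked mouse, adds the default Enhanced Input mapping and stores the BP_Unit returned by GetActorOfClass.
; The click action traces visibility under the cursor and writes the hit location to that unit's blackboard, leaving any movement to its AI.
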(event Input|EnhancedActionEvents|EnhancedInputActionIA_SetDestination_Click
  (params (ActionValue :type Boolean) (ElapsedSeconds :type Float%20%28double-precision%29) (TriggeredSeconds :type Float%20%28double-precision%29) (InputAction :type Input%20Action%20Object%20Reference :default "/Game/TopDown/Input/Actions/IA_SetDestination_Click.IA_SetDestination_Click"))
  (bind _hitresult (Game|Player|GetHitResultUnderCursorbyChannel "TraceTypeQuery1" true))
  (bind (_bblockinghit _binitialoverlap _time _distance _location) (Collision|BreakHitResult _hitresult))
  (:Triggered
    (if _bblockinghit
      (AI|Components|Blackboard|SetValueasVector (AI|GetBlackboard (Variables|Default|GetUnitControlled)) (Variables|Default|GetLocationBlackBoardKey) _location))))

(event EventBeginPlay
  (bind _returnvalue (PlayerController|LocalPlayerSubsystems|GetEnhancedInputLocalPlayerSubsystem))
  (Input|SetInputModeGameandUI self 0 "LockAlways" true false)
  (Utilities|IsValid _returnvalue
    (:Is%20Valid
      (Input|AddMappingContext _returnvalue "/Game/TopDown/Input/IMC_Default.IMC_Default" 0 "(bIgnoreAllPressedKeysUntilRelease=True,bForceImmediately=False)")
      (bind _returnvalue_2 (Actor|GetActorOfClass "/Game/Blueprints/BP_Unit.BP_Unit_C"))
      (Variables|Default|SetUnitControlled _returnvalue_2))))

(fn ConstructionScript)