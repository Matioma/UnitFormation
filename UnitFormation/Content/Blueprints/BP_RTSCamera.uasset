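; BP_RTSCamera is an RTS-style camera that becomes player 0's view target on BeginPlay and pans with the mouse.
; Each Tick, MoveLeft, which pans in any direction despite its name, compares the cursor with the viewport center.
; Beyond the radial CameraTolerance, it moves DefaultSceneRoot toward the cursor at CameraSpeed scaled by delta time, mapping screen up to +X and right to +Y.
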(event EventBeginPlay
  (Game|Player|SetViewTargetwithBlend (Game|GetPlayerController 0) self 0.0 "VTBlend_Linear" 0.0 false))

(event EventTick
  (params (DeltaSeconds :type Float%20%28single-precision%29))
  (CallFunction|MoveLeft DeltaSeconds))

(fn ConstructionScript)

(fn MoveLeft
  (params (DeltaTime :type Float%20%28double-precision%29))
  (bind _returnvalue (Class|WidgetLayoutLibrary|GetMousePositiononViewport))
  (bind _screencenter (|ComputeScreenCenter))
  (|IsMouseTooFarFromCenter (|MovementDirection _screencenter _returnvalue)
    (:Yes
      (Transformation|AddRelativeLocation (Variables|Default|GetDefaultSceneRoot) (|ComputeCameraOffsetVector (|MovementDirection _screencenter _returnvalue) (* DeltaTime (Variables|Default|GetCameraSpeed))) false false))))