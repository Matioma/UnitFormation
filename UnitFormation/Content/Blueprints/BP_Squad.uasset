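; BP_Squad is a squad controller that sends units to a location in a line formation.
; On BeginPlay it gathers every BP_Unit in the level into SquadUnits.
; SentSquadToLocation writes each unit's destination to its Blackboard, spacing them along world X by DistanceBetween.
; FormationStartLocation adds half the formation length to the target's X, so the line extends onward from there rather than centering on it.
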(event Custom|SentSquadToLocation
  (params (Location :type Vector))
  (bind _newparam (CallFunction|FormationStartLocation Location))
  (for (_array_element _array_index) (Variables|Default|GetSquadUnits)
    (AI|Components|Blackboard|SetValueasVector (AI|GetBlackboard _array_element) (Variables|Default|GetLocationBlackBoardKey) (+ _newparam (Math|Vector|MakeVector (* (Variables|Default|GetDistanceBetween) _array_index) 0.0 0.0)))))

(event EventBeginPlay
  (bind _outactors (Actor|GetAllActorsOfClass "/Game/Blueprints/BP_Unit.BP_Unit_C"))
  (Variables|Default|SetSquadUnits _outactors))

(fn ConstructionScript)

(fn FormationStartLocation
  (params (B :type Vector))
  (return (+ (Math|Vector|MakeVector (/ (* (Utilities|Array|Length (Variables|Default|GetSquadUnits)) (Variables|Default|GetDistanceBetween)) 2.0) 0.0 0.0) B)))